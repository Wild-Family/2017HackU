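; BP_Shell is a fireworks shell actor that climbs until it passes a height limit, then removes itself.
; Each Tick offsets the root component along its local Z by ShellSpeed scaled by delta time, without sweep or physics.
; It destroys itself once its world Z reaches a hard-coded ceiling, with no burst effect in this graph.
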(event `self.ReceiveTick`
  (params (DeltaSeconds :type "Float (single-precision)"))
  (`SceneComponent.K2_AddLocalOffset` (`self.DefaultSceneRoot`) (`KismetMathLibrary.MakeVector` 0.0 0.0 (* DeltaSeconds (`self.shellSpeed`))) false false)
  (if (>= (.z (.location (`self.GetTransform`))) 10000.0)
    (`self.K2_DestroyActor`)))

(fn `UserConstructionScript`)