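; BP_Shell1 is a firework shell actor that launches upward and is replaced by another actor at a set altitude.
; BeginPlay waits through a fixed delay, then sets a Start flag and plays a launch sound at the shell's location.
; Once started, Tick moves the root along local Z, scaled by ShellSpeed and delta time.
; At the height threshold it spawns Rand_col at its transform and destroys itself.
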(event `self.ReceiveBeginPlay`
  (`KismetSystemLibrary.Delay` 10.0)
  (set `self.start` true)
  (`GameplayStatics.PlaySoundAtLocation` "/Game/Fireworks/launch_fadeout2.launch_fadeout2" (`self.K2_GetActorLocation`)))

(event `self.ReceiveTick`
  (params (DeltaSeconds :type "Float (single-precision)"))
  (if (`self.start`)
    (`SceneComponent.K2_AddLocalOffset` (`self.DefaultSceneRoot`) (`KismetMathLibrary.MakeVector` 0.0 0.0 (* DeltaSeconds (`self.shellSpeed`))) false false)
    (if (>= (.z (.location (`self.GetTransform`))) 14000.0)
      (`|SpawnActorFromClass` "/Game/Fireworks/rand_col.rand_col_C" (`self.GetTransform`) "Undefined" "OverrideRootScale" null null)
      (`self.K2_DestroyActor`))))

(fn `UserConstructionScript`)